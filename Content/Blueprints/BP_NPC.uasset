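; BP_NPC is a dialogue NPC that loops a drunk idle animation and shows its lines one at a time.
; The IA_Talk input calls Interact on overlapping BP_npc actors that implement the BP_Dialogue interface.
; Each Interact advances TalkIndex, shows that Dialogue entry in a lazily created BP_DialogueUI widget and plays a 2D sound.
; Once the index passes the last line, the widget leaves its parent; the index never resets.
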(event Input|EnhancedActionEvents|EnhancedInputActionIA_Talk
  (params (ActionValue :type Boolean) (ElapsedSeconds :type Float%20%28double-precision%29) (TriggeredSeconds :type Float%20%28double-precision%29) (InputAction :type Input%20Action%20Object%20Reference :default "/Game/Input/InputAction/IA_Talk.IA_Talk"))
  (:Started
    (for _array_element (Collision|GetOverlappingActors "BP_npc_C" :!class /Script/Engine.Actor)
      (if (Utilities|DoesObjectImplementInterface _array_element "/Game/Blueprints/BP_Dialogue.BP_Dialogue_C")
        (CallFunction|Interact _array_element)))))

(event EventBeginPlay
  (Components|Animation|PlayAnimation (Variables|Default|GetSkeletalMesh) "/Game/Modern_woman_2/Animations/Drunk_Idle_Variation_Anim.Drunk_Idle_Variation_Anim" true))

(event EventInteract
  (params (Interactor :type Actor%20Object%20Reference))
  (Math|Integer|IncrementInt (Variables|Default|GettalkIndex)
    (:%20%20
      (if (< (Variables|Default|GettalkIndex) (Utilities|Array|Length (Variables|Default|Getdialogue)))
        (Variables|Default|GetUI
          (:then
            _)
          (:else
            (bind _returnvalue (UserInterface|CreateWidget "/Game/Blueprints/BP_DialogueUI.BP_DialogueUI_C" (Game|GetPlayerController 0)))
            (bind _output_get (Variables|Default|SetUI _returnvalue))
            (UserInterface|Viewport|AddtoViewport _output_get 0)))
        (Rendering|Components|TextRender|SetText (Variables|/Game/Blueprints/BP_DialogueUI.BP_DialogueUI_C|GetTextBlock_1 (Variables|Default|GetUI)) (Utilities|Text|ToText(String) (Utilities|Array|Get(acopy) (Variables|Default|Getdialogue) (Variables|Default|GettalkIndex))))
        (Audio|PlaySound2D 0 1.0 1.0 0.0 0 0)
        (else
          (Widget|RemovefromParent (Variables|Default|GetUI)))))))

(fn ConstructionScript)